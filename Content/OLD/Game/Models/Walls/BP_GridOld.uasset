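; Legacy grid room generator that, on BeginPlay, is meant to build a small walled floor with doors and occupants.
; It spawns floor tiles, uses MakeWall for inward-facing edges and corners, then picks random walls for doors.
; It then places or moves the player, rolls for a chest and spawns enemies, marking tile occupancy.
; Several links are broken: inner floor loop, tile-array adds and wall removal never run, and some references are missing.
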(event Custom|SpawnPlayer
  (bind (_tileclass _tilelocation) (Utilities|Struct|Break))
  (bind _returnvalue (Pawn|GetController))
  ;[1 1 1] spawn player
  (bind _outactors (Actor|GetAllActorsOfClass 0))
  (Variables|Default|SetStartingTile (Utilities|Array|Get(acopy) (Variables|Default|GetFloorTiles) (* (Variables|Default|GetX%20Tiles) (/ (Variables|Default|GetY%20Tiles) 2))))
  (if (Utilities|IsValid (Utilities|Array|Get(acopy) _outactors))
    ;;[1 1 1] use old player if one exists
    (AI|Navigation|SimpleMovetoActor _returnvalue _tileclass)
    (Variables|Default|Setoccupant _tileclass _returnvalue)
    (else
      ;;[1 1 1] spawn new player if null
      (bind _returnvalue_2 (Game|SpawnActorfromClass 0 (Math|Conversions|ToTransform(Vector) _tilelocation) "AlwaysSpawn" 0))
      (Variables|Default|SetSpawnedPlayer 0 _returnvalue_2)
      (Variables|Default|Setoccupant _tileclass (Pawn|GetController _returnvalue_2))))
  (Variables|Default|SetbOccupied _tileclass true))

(event EventBeginPlay
  (bind _tileclass (Utilities|Struct|Break))
  (bind _returnvalue (Transformation|GetActorLocation))
  (bind _tilesize (Variables|Default|GetTileSize))
  (bind _tilesize_2 (Variables|Default|GetTileSize))
  (bind _tilesize_3 (Variables|Default|GetTileSize))
  (bind _tilesize_4 (Variables|Default|GetTileSize))
  (bind _walltiles (Variables|Default|GetWallTiles))
  (bind _returnvalue_2 (* _tilesize_2 -1))
  (Variables|Default|SetY%20Tiles 4)
  (Variables|Default|SetX%20Tiles 4)
  (Variables|Default|SetMaxDoors (/ (* (* (Variables|Default|GetX%20Tiles) 2) (* (Variables|Default|GetY%20Tiles) 2)) 16))
  (Variables|Default|SetStartingTile "")
  (Utilities|FlowControl|Sequence
    (:then_0
      ;[1 1 1] Create Floor
      (Utilities|Array|Clear (Variables|Default|GetFloorTiles))
      (for _index (range 0 (- (Variables|Default|GetX%20Tiles) 1))
        (bind _returnvalue_3 (Game|SpawnActorfromClass (.FloorClass (Variables|Default|GetFloorClass)) (Math|Transform|MakeTransform (Math|Vector|MakeVector (+ (* _index (Math|Conversions|ToFloat(Integer) (Variables|Default|GetTileSize))) (.x _returnvalue)) (.y _returnvalue) (.z _returnvalue))) "Undefined" 0))))
    (:then_1
      (for _array_element (Variables|Default|GetFloorTiles)
        ;[1 1 1] Create walls
        (Utilities|FlowControl|Sequence
          (:then_0
            (if (== (.Row (Utilities|Struct|Break _array_element)) 0)
              (CallFunction|MakeWall (.TileClass (Utilities|Struct|Break _array_element)) (* (Variables|Default|GetTileSize) -1) 0 (.WallClass (Variables|Default|GetWallClass)) true)))
          (:then_1
            (if (== (.Column (Utilities|Struct|Break _array_element)) 0)
              (CallFunction|MakeWall (.TileClass (Utilities|Struct|Break _array_element)) 0 (* (Variables|Default|GetTileSize) -1) (.WallClass (Variables|Default|GetWallClass)) true)))
          (:then_2
            (if (== (.Row (Utilities|Struct|Break _array_element)) (- (Variables|Default|GetX%20Tiles) 1))
              (CallFunction|MakeWall (.TileClass (Utilities|Struct|Break _array_element)) (Variables|Default|GetTileSize) 0 (.WallClass (Variables|Default|GetWallClass)) true)))
          (:then_3
            (if (== (.Column (Utilities|Struct|Break _array_element)) (- (Variables|Default|GetY%20Tiles) 1))
              (CallFunction|MakeWall (.TileClass (Utilities|Struct|Break _array_element)) 0 (Variables|Default|GetTileSize) (.WallClass (Variables|Default|GetWallClass)) true)))
          (:then_4
            (if (and (== (.Row (Utilities|Struct|Break _array_element)) 0) (== (.Column (Utilities|Struct|Break _array_element)) 0))
              (CallFunction|MakeWall (.TileClass (Utilities|Struct|Break _array_element)) _returnvalue_2 _returnvalue_2 (.CornerClass (Variables|Default|GetCornerClass)) false)))
          (:then_5
            (if (and (== (.Row (Utilities|Struct|Break _array_element)) 0) (== (.Column (Utilities|Struct|Break _array_element)) (- (Variables|Default|GetY%20Tiles) 1)))
              (CallFunction|MakeWall (.TileClass (Utilities|Struct|Break _array_element)) (* _tilesize_3 -1) _tilesize_3 (.CornerClass (Variables|Default|GetCornerClass)) false)))
          (:then_6
            (if (and (== (.Column (Utilities|Struct|Break _array_element)) 0) (== (.Row (Utilities|Struct|Break _array_element)) (- (Variables|Default|GetX%20Tiles) 1)))
              (CallFunction|MakeWall (.TileClass (Utilities|Struct|Break _array_element)) _tilesize_4 (* _tilesize_4 -1) (.CornerClass (Variables|Default|GetCornerClass)) false)))
          (:then_7
            (Development|PrintString (Utilities|String|Append (Utilities|String|ToString(Integer) (.Row (Utilities|Struct|Break _array_element))) "-" (Utilities|String|ToString(Integer) (.Column (Utilities|Struct|Break _array_element)))))
            (if (and (== (.Row (Utilities|Struct|Break _array_element)) (- (Variables|Default|GetX%20Tiles) 1)) (== (.Column (Utilities|Struct|Break _array_element)) (- (Variables|Default|GetY%20Tiles) 1)))
              (CallFunction|MakeWall (.TileClass (Utilities|Struct|Break _array_element)) _tilesize _tilesize (.CornerClass (Variables|Default|GetCornerClass)) false)))))
      (for _index_2 (range 1 (Variables|Default|GetMaxDoors))
        (Variables|Default|SetTempDoorIndex (Math|Random|RandomIntegerinRange 0 (- (Utilities|Array|Length _walltiles) 1)))
        (if (not (== (Utilities|GetClass (.tileclass (Utilities|Array|Get(acopy) _walltiles (Variables|Default|GetTempDoorIndex)))) 0))
          (Utilities|FlowControl|Sequence
            (:then_0
              (if (not (== (Variables|Default|GetDefaultSceneRoot (.tileclass (Utilities|Array|Get(acopy) _walltiles (Variables|Default|GetTempDoorIndex)))) 0))
                (bind _output_get (Variables|Default|SetTempDoorTransform (Transformation|GetWorldTransform (Variables|Default|GetDefaultSceneRoot (.tileclass (Utilities|Array|Get(acopy) _walltiles (Variables|Default|GetTempDoorIndex)))))))
                (bind _returnvalue_4 (Game|SpawnActorfromClass (.DoorClass (Variables|Default|GetDoorClass)) _output_get "Undefined" 0)))))))
      (Variables|Default|SetStartingIndex (/ (* (Variables|Default|GetX%20Tiles) (Variables|Default|GetY%20Tiles)) 2))
      (CallFunction|SpawnPlayer)
      (Utilities|FlowControl|Sequence
        (:then_1
          ;[1 1 1] add Chest
          (if (>= (Math|Random|RandomIntegerinRange 0 100) 75)
            (bind _returnvalue_5 (Game|SpawnActorfromClass 0 (Math|Conversions|ToTransform(Vector) (Utilities|Struct|Break)) "AdjustIfPossibleButAlwaysSpawn" 0))
            (Variables|Default|Setoccupant _tileclass _returnvalue_5)
            (Variables|Default|SetbOccupied _tileclass true)))
        (:then_2
          ;[1 1 1] add AI
          (for _index_3 (range 0 (+ (/ (Variables|Default|GetMaxDoors) 2) 1))
            (CallFunction|SpawnEnemy)))))))

(fn ConstructionScript)

(fn MakeWall
  (params (EdgeActor :type %20Object%20Reference) (X%20Offset :type Integer) (Y%20Offset :type Integer) (TileClass :type %20Class%20Reference) (bRotate :type Boolean))
  (bind _returnvalue (Transformation|GetActorLocation EdgeActor))
  (bind (_x _y _z) (Math|Vector|BreakVector _returnvalue))
  (bind _returnvalue_2 (Game|SpawnActorfromClass TileClass (Math|Transform|MakeTransform (Math|Vector|MakeVector (+ _x (Math|Conversions|ToFloat(Integer) X%20Offset)) (+ _y (Math|Conversions|ToFloat(Integer) Y%20Offset)) _z)) "Undefined" 0))
  (if bRotate
    (Transformation|SetActorRotation _returnvalue_2 (Math|Rotator|FindLookatRotation (Transformation|GetActorLocation _returnvalue_2) (Transformation|GetActorLocation EdgeActor)))))

(fn SpawnEnemy
  (bind _asbp_tile_floor (Utilities|Casting|CastTo (Utilities|Struct|Break)))
  (if (not (Variables|Default|GetbOccupied _asbp_tile_floor))
    (bind _returnvalue (Game|SpawnActorfromClass 0 (Math|Conversions|ToTransform(Vector) (Transformation|GetActorLocation _asbp_tile_floor)) "AlwaysSpawn" 0))
    (Variables|Default|Setoccupant _asbp_tile_floor _returnvalue)
    (Variables|Default|SetbOccupied _asbp_tile_floor true)))