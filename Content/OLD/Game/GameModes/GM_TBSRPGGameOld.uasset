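; Legacy game mode for a turn-based RPG that sets up the map and player pawns and alternates turns.
; On BeginPlay it clears actors, has a child actor generate the grid, then spawns and registers each player with the controller at the first PlayerStart.
; SetStart teleports existing pawns to that start and resets their turns.
; EndTurn toggles player and AI turns, but the AI turn immediately passes back to the player.
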(event EventBeginPlay
  (CallFunction|ResetMap 0 0 0)
  (for _index (range 1 (Variables|Default|GetCurrentPlayersAmount))
    (bind _outactors (Actor|GetAllActorsOfClass "/Script/Engine.PlayerStart"))
    (bind _returnvalue (Game|SpawnActorfromClass 0 (Math|Conversions|ToTransform(Vector) (Transformation|GetActorLocation (Utilities|Array|Get(acopy) _outactors))) "AlwaysSpawn" 0))
    (bind _astbsplayer_controller (Utilities|Casting|CastTo (Game|GetPlayerController 0)))
    (CallFunction|AddPlayer _astbsplayer_controller _returnvalue)
    (CallFunction|SelectPlayer _astbsplayer_controller _returnvalue)))

(fn ConstructionScript)

(fn SetStart
  (bind _outactors (Actor|GetAllActorsOfClass 0))
  (bind _outactors_2 (Actor|GetAllActorsOfClass "/Script/Engine.PlayerStart"))
  ;[1 1 1] Move Players outside map
  (for _array_element _outactors
    (Transformation|Teleport _array_element (Transformation|GetActorLocation (Utilities|Array|Get(acopy) _outactors_2)) "0, 0, 0")
    ;[1 1 1] Reset Player Pawns
    (CallFunction|ResetTurn _array_element)))

(fn ResetMap
  (params (Side :type Byte) (Last :type Byte) (Next :type Byte))
  (Utilities|FlowControl|Sequence
    (:then_0
      (Actor|GetAllActorsOfClass 0)
      (for _array_element 0
        (Actor|DestroyActor _array_element)))
    (:then_1
      (bind _outactors (Actor|GetAllActorsOfClass 0))
      (for _array_element_2 _outactors
        (Actor|DestroyActor _array_element_2)))
    (:then_2
      (bind _outactors_2 (Actor|GetAllActorsOfClass 0))
      (for _array_element_3 _outactors_2
        (Actor|DestroyActor _array_element_3)))
    (:then_3
      (bind _outactors_3 (Actor|GetAllActorsOfClass 0))
      (for _array_element_4 _outactors_3
        (Actor|DestroyActor _array_element_4)))
    (:then_4
      (bind _asbp_grid_gen (Utilities|Casting|CastTo (Variables|/Script/Engine.ChildActorComponent|GetChildActor (Variables|Default|GetChildActor))))
      (bind _tiles (CallFunction|GenerateGrid _asbp_grid_gen 0 0))
      (Variables|Default|SettileGrid 0 _tiles)
      (CallFunction|SetStart))))

(fn EndTurn
  (if (Variables|Default|GetbPlayerTurn)
    (CallFunction|ResetAITurn)
    (else
      (CallFunction|ResetPlayerTurn))))

(fn ResetPlayerTurn
  (Variables|Default|SetbPlayerTurn true)
  (bind _astbsplayer_controller (Utilities|Casting|CastTo (Game|GetPlayerController 0))
    (:then
      (CallFunction|ResetTurn _astbsplayer_controller))
    (:CastFailed
      (Class|GameMode|EndMatch))))

(fn ResetAITurn
  (Variables|Default|SetbPlayerTurn false)
  (CallFunction|EndTurn))