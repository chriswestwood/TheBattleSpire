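; Older grid generator that builds a randomly sized rectangular floor of tile actors from the current and next floor types and returns them.
; GenerateGrid picks edge types, with north taking the next type and others random, weighted toward the current one.
; It spawns tiles with random height jitter, links neighbours and gives border tiles a secondary type.
; It then marks randomly placed side openings and two-tile-deep walls before calling StartSetup on each tile.
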(event EventBeginPlay)

(fn ConstructionScript)

(fn ClearGrid
  (Utilities|Array|Clear (.Tiles (Variables|Default|GetTiles))))

(fn GenerateGrid
  (params (CurrentFloorType :type Byte) (NextFloorType :type Byte))
  (CallFunction|ClearGrid)
  (CallFunction|GenerateTypes CurrentFloorType NextFloorType)
  (CallFunction|GenerateGridSize)
  (CallFunction|SpawnGrid)
  (CallFunction|SetTilePositions)
  (CallFunction|SetGridTypes)
  (CallFunction|SetAccess)
  (CallFunction|SetWalls)
  (CallFunction|Startup)
  (return (.Tiles (Variables|Default|GetTiles))))

(fn GenerateTypes
  (params (NewCurrent :type Byte) (Previous :type Byte))
  (bind _returnvalue (Math|Random|RandomIntegerinRange 0 100))
  (bind _returnvalue_2 (|GetNumEnumEntries))
  (bind _tiletypepercentchance (Variables|Default|GetTileTypePercentChance))
  (bind _returnvalue_3 (<= _returnvalue _tiletypepercentchance))
  (bind _returnvalue_4 (- _returnvalue_2 1))
  (bind _returnvalue_5 (Math|Random|RandomIntegerinRange 0 _returnvalue_4))
  (bind _returnvalue_6 (Math|Conversions|ToByte(Integer) _returnvalue_5))
  (bind _returnvalue_7 (Utilities|Enum|ByteToEnumObject _returnvalue_6))
  (Variables|Default|SetmiddleType NewCurrent)
  (Variables|Default|SetnorthType Previous)
  (if _returnvalue_3
    (Variables|Default|SeteastType NewCurrent)
    (else
      (Variables|Default|SeteastType _returnvalue_7)))
  (if _returnvalue_3
    (Variables|Default|SetsouthType NewCurrent)
    (else
      (Variables|Default|SetsouthType _returnvalue_7)))
  (if _returnvalue_3
    (Variables|Default|SetwestType NewCurrent)
    (else
      (Variables|Default|SetwestType _returnvalue_7))))

(fn GenerateGridSize
  (bind (_1 _2) (CallFunction|GetRandomXY))
  (if (Math|Random|RandomBool)
    (Variables|Default|SetxSize _1)
    (Variables|Default|SetySize _2)
    (else
      (Variables|Default|SetxSize _2)
      (Variables|Default|SetySize _1))))

(fn SpawnGrid
  (for _index (range 1 (Variables|Default|GetySize))
    (for _index_2 (range 1 (Variables|Default|GetxSize))
      (bind _returnvalue (Game|SpawnActorfromClass 0 (Math|Transform|MakeTransform (+ (* (Math|Vector|MakeVector (Math|Conversions|ToFloat(Integer) _index) (Math|Conversions|ToFloat(Integer) _index_2) 0.0) "100.000000,100.000000,0.000000") (Math|Vector|MakeVector 0.0 0.0 (Math|Conversions|ToFloat(Integer) (Math|Random|RandomIntegerinRange 0 50))))) "Undefined" 0))
      (CallFunction|SetLocation _returnvalue _index_2 _index)
      (Utilities|Array|Add (.Tiles (Variables|Default|GetTiles)) _returnvalue)))
  (return))

(fn SetGridTypes
  (for _array_element (.Tiles (Variables|Default|GetTiles))
    (Variables|Default|SetType1 _array_element (Variables|Default|GetmiddleType))
    (Utilities|FlowControl|Sequence
      (:then_0
        (if (<= (Variables|Default|GetXLoc _array_element) 2)
          (CallFunction|SetType2 _array_element (Variables|Default|GetwestType))))
      (:then_1
        (if (>= (Variables|Default|GetXLoc _array_element) (- (Variables|Default|GetxSize) 1))
          (CallFunction|SetType2 _array_element (Variables|Default|GeteastType))))
      (:then_2
        (if (<= (Variables|Default|GetYLoc _array_element) 2)
          (CallFunction|SetType2 _array_element (Variables|Default|GetnorthType))))
      (:then_3
        (if (>= (Variables|Default|GetYLoc _array_element) (- (Variables|Default|GetySize) 1))
          (CallFunction|SetType2 _array_element (Variables|Default|GetsouthType)))))))

(fn GetRandomXY
  (bind _returnvalue (Math|Random|RandomIntegerinRange 15 30))
  (return (Class|KismetSystemLibrary|MakeLiteralInteger _returnvalue) (Class|KismetSystemLibrary|MakeLiteralInteger (Math|Random|RandomIntegerinRange 10 (- 50 _returnvalue)))))

(fn SetAccess
  (if (Utilities|Enum|Equal(Enum) 0 0)
    (LocalVariables|SetnorthSize 2)
    (LocalVariables|SetsouthSize 2)
    (LocalVariables|SetwestSize 2)
    (LocalVariables|SeteastSize 2)
    (else
      (if (Utilities|Enum|Equal(Enum) 0 0)
        (LocalVariables|SetnorthSize 2)
        (else
          (LocalVariables|SetnorthSize (Math|Random|RandomIntegerinRange 2 (- (Variables|Default|GetxSize) 5)))))
      (if (Utilities|Enum|Equal(Enum) 0 0)
        (LocalVariables|SetsouthSize 2)
        (else
          (LocalVariables|SetsouthSize (Math|Random|RandomIntegerinRange 2 (- (Variables|Default|GetxSize) 5)))))
      (if (Utilities|Enum|Equal(Enum) 0 0)
        (LocalVariables|SetwestSize 2)
        (else
          (LocalVariables|SetwestSize (Math|Random|RandomIntegerinRange 2 (- (Variables|Default|GetySize) 5)))))
      (if (Utilities|Enum|Equal(Enum) 0 0)
        (LocalVariables|SeteastSize 2)
        (else
          (LocalVariables|SeteastSize (Math|Random|RandomIntegerinRange 2 (- (Variables|Default|GetySize) 5)))))))
  (LocalVariables|SetnorthStart (Math|Random|RandomIntegerinRange 3 (|((mapSize-2)-PathSize) (Variables|Default|GetxSize) (LocalVariables|GetnorthSize))))
  (LocalVariables|SetsouthStart (Math|Random|RandomIntegerinRange 3 (|((mapSize-2)-PathSize) (Variables|Default|GetxSize) (LocalVariables|GetsouthSize))))
  (LocalVariables|SetwestStart (Math|Random|RandomIntegerinRange 3 (|((mapSize-2)-PathSize) (Variables|Default|GetySize) (LocalVariables|GetwestSize))))
  (LocalVariables|SeteastStart (Math|Random|RandomIntegerinRange 3 (|((mapSize-2)-PathSize) (Variables|Default|GetySize) (LocalVariables|GeteastSize))))
  (for _array_element (.Tiles (Variables|Default|GetTiles))
    (Utilities|FlowControl|Sequence
      (:then_0
        ;[1 1 1] North
        (if (or (Utilities|Enum|Equal(Enum) 0 0) (Utilities|Enum|Equal(Enum) 0 0))
          (if (== (Variables|Default|GetYLoc _array_element) 1)
            (if (|(x==(start+(size/2))) (Variables|Default|GetXLoc _array_element) (LocalVariables|GetnorthStart) (LocalVariables|GetnorthSize))
              (CallFunction|SetAccess _array_element 0))
            (elif (<= (Variables|Default|GetYLoc _array_element) 3)
              (if (|((start<=x)&&(x<=(start+size))) (Variables|Default|GetXLoc _array_element) (LocalVariables|GetnorthStart) (LocalVariables|GetnorthSize)) :!label _label
                (CallFunction|SetAccess _array_element 0))))
          (elif (<= (Variables|Default|GetYLoc _array_element) 2)
            (goto _label))))
      (:then_1
        ;[1 1 1] South
        (if (or (Utilities|Enum|Equal(Enum) 0 0) (Utilities|Enum|Equal(Enum) 0 0))
          (if (== (Variables|Default|GetYLoc _array_element) (Variables|Default|GetySize))
            (if (|(x==(start+(size/2))) (Variables|Default|GetXLoc _array_element) (LocalVariables|GetsouthStart) (LocalVariables|GetsouthSize))
              (CallFunction|SetAccess _array_element 0))
            (elif (>= (Variables|Default|GetYLoc _array_element) (- (Variables|Default|GetySize) 2))
              (if (|((start<=x)&&(x<=(start+size))) (Variables|Default|GetXLoc _array_element) (LocalVariables|GetsouthStart) (LocalVariables|GetsouthSize)) :!label _label_2
                (CallFunction|SetAccess _array_element 0))))
          (elif (>= (Variables|Default|GetYLoc _array_element) (- (Variables|Default|GetySize) 1))
            (goto _label_2))))
      (:then_2
        ;[1 1 1] West
        (if (or (Utilities|Enum|Equal(Enum) 0 0) (Utilities|Enum|Equal(Enum) 0 0))
          (if (== (Variables|Default|GetXLoc _array_element) 1)
            (if (|(x==(start+(size/2))) (Variables|Default|GetYLoc _array_element) (LocalVariables|GetwestStart) (LocalVariables|GetwestSize))
              (CallFunction|SetAccess _array_element 0))
            (elif (<= (Variables|Default|GetXLoc _array_element) 3)
              (if (|((start<=x)&&(x<=(start+size))) (Variables|Default|GetYLoc _array_element) (LocalVariables|GetwestStart) (LocalVariables|GetwestSize)) :!label _label_3
                (CallFunction|SetAccess _array_element 0))))
          (elif (<= (Variables|Default|GetXLoc _array_element) 2)
            (goto _label_3))))
      (:then_3
        ;[1 1 1] West
        (if (or (Utilities|Enum|Equal(Enum) 0 0) (Utilities|Enum|Equal(Enum) 0 0))
          (if (== (Variables|Default|GetXLoc _array_element) (Variables|Default|GetxSize))
            (if (|(x==(start+(size/2))) (Variables|Default|GetYLoc _array_element) (LocalVariables|GeteastStart) (LocalVariables|GeteastSize))
              (CallFunction|SetAccess _array_element 0))
            (elif (>= (Variables|Default|GetXLoc _array_element) (- (Variables|Default|GetxSize) 2))
              (if (|((start<=x)&&(x<=(start+size))) (Variables|Default|GetYLoc _array_element) (LocalVariables|GeteastStart) (LocalVariables|GeteastSize)) :!label _label_4
                (CallFunction|SetAccess _array_element 0))))
          (elif (>= (Variables|Default|GetXLoc _array_element) (- (Variables|Default|GetxSize) 1))
            (goto _label_4))))))
  (return))

(fn SetWalls
  (for _array_element (.Tiles (Variables|Default|GetTiles))
    (if (<= (Variables|Default|GetXLoc _array_element) 2)
      (Variables|Default|SetExitNum _array_element 0)
      (CallFunction|SetAccess _array_element 0 :!label _label)
      (elif (>= (Variables|Default|GetXLoc _array_element) (- (Variables|Default|GetxSize) 1))
        (Variables|Default|SetExitNum _array_element 0)
        (goto _label)
        (elif (<= (Variables|Default|GetYLoc _array_element) 2)
          (Variables|Default|SetExitNum _array_element 0)
          (goto _label)
          (elif (>= (Variables|Default|GetYLoc _array_element) (- (Variables|Default|GetySize) 1))
            (Variables|Default|SetExitNum _array_element 0)
            (goto _label))))))
  (return))

(fn Startup
  (for _array_element (.Tiles (Variables|Default|GetTiles))
    (CallFunction|StartSetup _array_element))
  (return))

(fn SetTilePositions
  (bind _tiles (Variables|Default|GetTiles))
  (for (_array_element _array_index) _tiles
    (Utilities|FlowControl|Sequence
      (:then_0
        (if (> _array_index (Variables|Default|GetxSize))
          (Variables|Default|Setnorth _array_element (Utilities|Array|Get(acopy) _tiles (- _array_index (Variables|Default|GetxSize))))))
      (:then_1
        (if (<= _array_index (- (Utilities|Array|Length _tiles) (Variables|Default|GetxSize)))
          (Variables|Default|Setsouth _array_element (Utilities|Array|Get(acopy) _tiles (+ _array_index (Variables|Default|GetxSize))))))
      (:then_2
        (if (!= (Variables|Default|GetXLoc _array_element) 1)
          (Variables|Default|Seteast _array_element (Utilities|Array|Get(acopy) _tiles (- _array_index 1)))))
      (:then_3
        (if (!= (Variables|Default|GetXLoc _array_element) (Variables|Default|GetxSize))
          (Variables|Default|Setwest _array_element (Utilities|Array|Get(acopy) _tiles (+ _array_index 1)))))))
  (return))