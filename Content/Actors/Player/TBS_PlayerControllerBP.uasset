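; Player controller for a turn-based game that handles mouse selection and movement of player pawns during the player's turn.
; Left click traces under the cursor and selects actors, making player pawns current; occupied tiles call SelectActor without an actor.
; Right click sends the current pawn along the path of an unoccupied, selectable tile, hit directly or via an actor.
; Both clicks then refresh that pawn's movement tiles; construction caches all pawns, and SelectTile is an empty stub.
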(event Input|MouseEvents|LeftMouseButton
  (params (Key :type Key%20Structure))
  (bind (_worldlocation _worlddirection) (Game|Player|ConvertMouseLocationToWorldSpace))
  ;[1 1 1] Select Target
  (:Pressed
    (Utilities|FlowControl|Sequence
      (:then_0
        (if (Variables|Default|GetisTurn)
          (bind (_outhit _returnvalue) (Collision|LineTraceByChannel _worldlocation (+ _worldlocation (* _worlddirection 10000)) "TraceTypeQuery1" false 0 "None"))
          (if _returnvalue
            (bind _astbs_tile_bp (Utilities|Casting|CastToTBS_TileBP (.HitActor (Collision|BreakHitResult _outhit)))
              (:then
                (bind _isocc (Default|IsOccupied _astbs_tile_bp))
                (if _isocc
                  (CallFunction|SelectActor)))
              (:CastFailed
                (bind _astbs_actor_bp (Utilities|Casting|CastToTBS_ActorBP (.HitActor (Collision|BreakHitResult _outhit))))
                (CallFunction|SelectActor _astbs_actor_bp))))))
      (:then_1
        (CallFunction|UpdateSelected)))))

(event Input|MouseEvents|RightMouseButton
  (params (Key :type Key%20Structure))
  (bind (_worldlocation _worlddirection) (Game|Player|ConvertMouseLocationToWorldSpace))
  ;[1 1 1] Action Target
  (:Pressed
    (Utilities|FlowControl|Sequence
      (:then_0
        (if (Variables|Default|GetisTurn)
          (bind (_outhit _returnvalue) (Collision|LineTraceByChannel _worldlocation (+ _worldlocation (* _worlddirection 10000)) "TraceTypeQuery1" false 0 "None"))
          (if _returnvalue
            (bind _astbs_tile_bp (Utilities|Casting|CastToTBS_TileBP (.HitActor (Collision|BreakHitResult _outhit)))
              (:then
                (bind _isocc (Default|IsOccupied _astbs_tile_bp))
                (if (and (not _isocc) (Variables|/Game/Actors/Grid/TBS_TileBP.TBS_TileBP_C|GetcanSelect _astbs_tile_bp))
                  (Default|MovetoTile (Variables|Default|GetCurrentPlayer) (Variables|/Game/Actors/Grid/TBS_TileBP.TBS_TileBP_C|GetTilePath _astbs_tile_bp))))
              (:CastFailed
                (bind _astbs_actor_bp (Utilities|Casting|CastToTBS_ActorBP (.HitActor (Collision|BreakHitResult _outhit))))
                (bind _isocc_2 (Default|IsOccupied (Variables|/Game/Actors/TBS_ActorBP.TBS_ActorBP_C|GetCurrentTile _astbs_actor_bp)))
                (if (and (not _isocc_2) (Variables|/Game/Actors/Grid/TBS_TileBP.TBS_TileBP_C|GetcanSelect (Variables|/Game/Actors/TBS_ActorBP.TBS_ActorBP_C|GetCurrentTile _astbs_actor_bp)))
                  (Default|MovetoTile (Variables|Default|GetCurrentPlayer) (Variables|/Game/Actors/Grid/TBS_TileBP.TBS_TileBP_C|GetTilePath (Variables|/Game/Actors/TBS_ActorBP.TBS_ActorBP_C|GetCurrentTile _astbs_actor_bp)))))))))
      (:then_1
        (CallFunction|UpdateSelected)))))

(fn ConstructionScript
  (bind _outactors (Actor|GetAllActorsOfClass "/Game/Actors/TBS_PawnBP.TBS_PawnBP_C"))
  (Variables|Default|SetPlayerPawns _outactors))

(fn SelectTile)

(fn SelectPlayer
  (params (SelectedPlayer :type TBS%20Player%20Pawn%20BP%20Object%20Reference))
  (bind _output_get (Variables|Default|SetCurrentPlayer SelectedPlayer))
  (Default|Select _output_get))

(fn SelectActor
  (params (InActor :type TBS%20Actor%20BP%20Object%20Reference))
  (bind _astbs_player_pawn_bp (Utilities|Casting|CastToTBS_PlayerPawnBP InActor)
    (:then
      (CallFunction|SelectPlayer _astbs_player_pawn_bp))
    (:CastFailed
      (Variables|Default|SetSelectedActor InActor))))

(fn UpdateSelected
  (bind _currentplayer (Variables|Default|GetCurrentPlayer))
  (if (Utilities|IsValid _currentplayer)
    (Default|GetMovementTiles _currentplayer)))