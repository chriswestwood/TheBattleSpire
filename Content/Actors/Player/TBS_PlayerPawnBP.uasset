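; Player-controlled pawn for a turn-based strategy game that can be selected and shows where it can move on the grid.
; Select, allowed only while MovementRange remains above zero, deselects every player pawn and turns this pawn's base green.
; GetMovementTiles has the game mode's GridSystem reset tiles, flood an area from the current tile by movement range with occupants blocking, and mark tiles selectable.
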(event EventSelect
  (if (> (Variables|Default|GetMovementRange) 0)
    (bind _outactors (Actor|GetAllActorsOfClass "TBS_PlayerPawnBP_C"))
    (for _array_element _outactors
      (Default|Deselect _array_element))
    (Rendering|Material|SetMaterial (Variables|Default|GetBase) 0 "/Game/Materials/Mat_GreenMetal.Mat_GreenMetal")))

(fn ConstructionScript
  (|CallParentFunction))

(fn GetMovementTiles
  (bind _astbs_game_mode_bp (Utilities|Casting|CastToTBS_GameModeBP (Game|GetGameMode)))
  (Default|ResetTiles (Variables|/Game/TBS_GameModeBP.TBS_GameModeBP_C|GetGridSystem _astbs_game_mode_bp))
  (Default|SelectAOETiles (Variables|/Game/TBS_GameModeBP.TBS_GameModeBP_C|GetGridSystem _astbs_game_mode_bp) (Variables|Default|GetCurrentTile) (Utilities|Array|MakeArray) (Variables|Default|GetMovementRange) true false)
  (Default|SetTilesSelectable (Variables|/Game/TBS_GameModeBP.TBS_GameModeBP_C|GetGridSystem _astbs_game_mode_bp)))