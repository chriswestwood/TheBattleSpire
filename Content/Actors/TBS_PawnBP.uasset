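; Turn-based strategy pawn Blueprint that can be selected, moved between tiles, and shows a health, armour and magic shield bar.
; On BeginPlay it places the life bar widget at the top of the pawn mesh's bounds and pushes the stats to it.
; Select and Deselect swap the base material between red and silver metal.
; MovetoTile, marked as test, claims the path's last tile and, on success, teleports straight to its occupant location.
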(event EventBeginPlay
  (bind _pawn (Variables|Default|GetPawn))
  (Transformation|SetRelativeLocation (Variables|Default|GetTBS_WidgetLifeBar) (Math|Vector|MakeVector 0.0 0.0 (+ (.Z (Math|Vector|BreakVector (Variables|/Script/Engine.SceneComponent|GetRelativeLocation _pawn))) (.Z (Math|Vector|BreakVector (.Max (Components|StaticMesh|GetLocalBounds _pawn)))))) false true)
  (CallFunction|SetStats))

(event Collision|EventActorBeginOverlap
  (params (OtherActor :type Actor%20Object%20Reference)))

(event EventTick
  (params (DeltaSeconds :type Float%20%28single-precision%29)))

(event EventSelect
  (Rendering|Material|SetMaterial (Variables|Default|GetBase) 0 "/Game/Materials/Mat_RedMetal.Mat_RedMetal"))

(event EventDeselect
  (Rendering|Material|SetMaterial (Variables|Default|GetBase) 0 "/Game/Materials/Mat_SilverMetal.Mat_SilverMetal"))

(event EventMovetoTile
  (params (inTiles :type Array%20of%20TBS%20Tile%20BP%20Object%20References))
  (bind _returnvalue (Utilities|Array|LastIndex inTiles))
  (bind _output (Utilities|Array|Get(acopy) inTiles _returnvalue))
  ;[1 1 1] MoveToPosition
  ;;[1 1 1] TEST
  (bind _bmoved (CallFunction|SetNewTile _output))
  (if _bmoved
    (Transformation|SetWorldLocation (Variables|Default|GetBase) (Transformation|GetWorldLocation (Variables|/Game/Actors/Grid/TBS_TileBP.TBS_TileBP_C|GetOccupantLocation _output)) false true)))

(fn ConstructionScript)

(fn SetStats
  (Default|UpdateStats (Variables|Default|GetTBS_WidgetLifeBar) (Variables|Default|GetHealth) (Variables|Default|GetArmour) (Variables|Default|GetMagicShield)))