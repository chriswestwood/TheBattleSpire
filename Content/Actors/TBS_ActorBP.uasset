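; Base tile-occupying actor with movement, selection and fall-to-destroy behavior.
; SetNewTile claims the target tile through SetOccupant and, only on success, releases the current tile and stores the new one.
; MoveToLoc sets the actor location directly, while Select, Deselect and MoveToTile are empty stubs.
; Fall sets IsFalling and runs a timeline that lowers the Base component a fixed step each update, then destroys the actor.
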(event Custom|Fall
  (bind _base (Variables|Default|GetBase))
  (bind _returnvalue (Transformation|GetWorldLocation _base))
  (bind (_x _y _z) (Math|Vector|BreakVector _returnvalue))
  ;[1 1 1] Fall (Destroy Actor)
  (Variables|Default|SetisFalling true)
  (Timeline|Timeline_1 PlayFromStart
    (:Update
      (Transformation|SetWorldLocation (Variables|Default|GetBase) (Math|Vector|MakeVector _x _y (- _z 5.0)) false true))
    (:Finished
      (Actor|DestroyActor))))

(event EventBeginPlay)

(event Collision|EventActorBeginOverlap
  (params (OtherActor :type Actor%20Object%20Reference)))

(fn ConstructionScript)

(fn MovetoLoc
  (params (NewLoc :type Vector))
  (Transformation|SetActorLocation NewLoc false false))

(fn Select)

(fn Deselect)

(fn MovetoTile
  (params (inTiles :type Array%20of%20TBS%20Tile%20BP%20Object%20References)))

(fn SetNewTile
  (params (NewTIle :type TBS%20Tile%20BP%20Object%20Reference%20%28by%20ref%29))
  (bind _bupdated (Default|SetOccupant NewTIle self))
  (if _bupdated
    (Default|RemoveOccupant (Variables|Default|GetCurrentTile))
    (Variables|Default|SetCurrentTile NewTIle)
    (return true)
    (else
      (return false))))