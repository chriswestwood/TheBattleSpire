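; Grid tile actor for the turn-based game that tracks one occupant and shows selectable and hover visuals, with hover only on the player's turn.
; It starts at a random height, and timelines animate height changes while moving the occupant along.
; A height of zero or less makes it fall with its occupant after a random delay, then the GameMode's GridSystem removes it.
; Clicks call an empty SelectTile event.
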(event Custom|MoveToNewHeight
  (params (NewHeight :type Integer))
  (bind _tile (Variables|Default|GetTile))
  (bind _returnvalue (Transformation|GetWorldLocation _tile))
  (bind (_x _y) (Math|Vector|BreakVector _returnvalue))
  ;[1 1 1] Change Height
  (if (not (Variables|Default|GetisFalling))
    (bind _output_get (Variables|Default|SetHeight NewHeight))
    (if (> _output_get 0)
      (Variables|Default|SetOldHeight (.Z (Math|Vector|BreakVector (Transformation|GetWorldLocation (Variables|Default|GetTile)))))
      (bind _newtrack_0 (Timeline|Timeline_0 PlayFromStart)
        (:Update
          (Transformation|SetWorldLocation _tile (Math|Vector|MakeVector _x _y (Math|Float|Lerp (Variables|Default|GetOldHeight) (* (Variables|Default|GetHeight) 1e+01) _newtrack_0)) false false)
          (if (Utilities|IsValid (Variables|Default|GetOccupant))
            (Default|MovetoLoc (Variables|Default|GetOccupant) (Transformation|GetWorldLocation (Variables|Default|GetOccupantLocation))))))
      (else
        (CallFunction|Fall)))))

(event Custom|SelectTile
  ;[1 1 1] Debug Select
)

(event Custom|Fall
  (bind _tile (Variables|Default|GetTile))
  (bind _occupant (Variables|Default|GetOccupant))
  (bind _returnvalue (Transformation|GetWorldLocation _tile))
  (bind _returnvalue_2 (Utilities|IsValid _occupant))
  (bind (_x _y _z) (Math|Vector|BreakVector _returnvalue))
  ;[1 1 1] Fall (Destroy Actor)
  (Variables|Default|SetisFalling true)
  (Audio|Components|Audio|Stop (Variables|Default|GetTimeline_0))
  (if _returnvalue_2
    (Variables|/Game/Actors/TBS_ActorBP.TBS_ActorBP_C|SetisFalling _occupant true))
  (Utilities|FlowControl|Delay (Math|Random|RandomFloatinRange 0.0 1.0))
  (if _returnvalue_2
    (Default|Fall (Variables|Default|GetOccupant))
    (Timeline|Timeline_1 PlayFromStart
      (:Update
        (Transformation|SetWorldLocation _tile (Math|Vector|MakeVector _x _y (- _z 1e+01)) false true))
      (:Finished
        (bind _astbs_game_mode_bp (Utilities|Casting|CastToTBS_GameModeBP (Game|GetGameMode)))
        (Default|RemoveTiles (Variables|/Game/TBS_GameModeBP.TBS_GameModeBP_C|GetGridSystem _astbs_game_mode_bp) (Utilities|Set|MakeSet self))))
    (else
      (Timeline|Timeline_1 PlayFromStart))))

(event MouseInput|EventActorOnClicked
  (params (ButtonPressed :type Key%20Structure))
  (CallFunction|SelectTile))

(event MouseInput|EventActorBeginCursorOver
  ;[1 1 1] Mouse Hover
  (CallFunction|Hover))

(event MouseInput|EventActorEndCursorOver
  ;[1 1 1] Mouse Hover
  (CallFunction|StopHover))

(event EventBeginPlay
  ;[1 1 1] BeginPlay
  (CallFunction|MovetoNewHeight (+ (Math|Random|RandomInteger 9) 1))
  (CallFunction|SetSelectable (Variables|Default|GetcanSelect)))

(fn ConstructionScript)

(fn Hover
  (if (Variables|Default|GetcanSelect)
    (bind _astbs_player_controller_bp (Utilities|Casting|CastToTBS_PlayerControllerBP (Game|GetPlayerController 0)))
    (if (Variables|/Game/Actors/Player/TBS_PlayerControllerBP.TBS_PlayerControllerBP_C|GetisTurn _astbs_player_controller_bp)
      (Rendering|SetVisibility (Variables|Default|GetHoverParticle) true false))))

(fn StopHover
  (Rendering|SetVisibility (Variables|Default|GetHoverParticle) false false))

(fn SetSelectable
  (params (isSelectable :type Boolean))
  (CallFunction|StopHover)
  (bind _output_get (Variables|Default|SetcanSelect isSelectable))
  (Rendering|SetVisibility (Variables|Default|GetSelectPlane) _output_get true))

(fn Destroy
  (Actor|DestroyActor))

(fn IsOccupied
  (return (Utilities|IsValid (Variables|Default|GetOccupant))))

(fn RemoveOccupant
  (Variables|Default|SetOccupant 0))

(fn SetOccupant
  (params (NewActor :type TBS%20Actor%20BP%20Object%20Reference))
  (if (Utilities|IsValid (Variables|Default|GetOccupant))
    (return false)
    (else
      (Variables|Default|SetOccupant NewActor)
      (return true))))