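; Grid system Blueprint that holds the set of tiles and selects them in area, line and facing-relative offset patterns.
; Area selection recurses through North/South/East/West neighbor links, storing each tile's path and pruning routes that are no shorter.
; All patterns feed SelectTile, which skips falling tiles, blocks on non-damageable occupants and applies occupant flags to damageable ones.
; Helpers make the selection selectable or reset tile states and paths.
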(fn ResetTiles
  (bind _result (Utilities|Set|ToArray (Variables|Default|GetTiles)))
  (for _array_element _result
    (Default|SetSelectable _array_element false)
    (Utilities|Array|Clear (Variables|/Game/Actors/Grid/TBS_TileBP.TBS_TileBP_C|GetTilePath _array_element)))
  (Utilities|Set|Clear (Variables|Default|GetSelectedTiles)))

(fn SelectAOETiles
  (params (CurrentTile :type TBS%20Tile%20BP%20Object%20Reference) (Path :type Array%20of%20TBS%20Tile%20BP%20Object%20References) (Count :type Integer) (Occupants%20Block :type Boolean) (Include%20Occupants :type Boolean))
  (bind _returnvalue (- Count 1))
  ;[1 1 1] always add first tile
  (if (== (Utilities|Array|Length Path) 0)
    ;[1 1 1] Add Tile to Selected
    (CallFunction|SelectTile CurrentTile Occupants%20Block Include%20Occupants)
    ;[1 1 1] Update Current Tile Path
    (LocalVariables|SetCurrentPath Path :!label _label)
    (Utilities|Array|Add (LocalVariables|GetCurrentPath) CurrentTile)
    (Variables|/Game/Actors/Grid/TBS_TileBP.TBS_TileBP_C|SetTilePath CurrentTile (LocalVariables|GetCurrentPath))
    ;[1 1 1] Check Next Tiles
    (if (>= _returnvalue 0)
      (Utilities|FlowControl|Sequence
        (:then_0
          (CallFunction|SelectAOETiles (Variables|/Game/Actors/Grid/TBS_TileBP.TBS_TileBP_C|GetNorth CurrentTile) (LocalVariables|GetCurrentPath) _returnvalue false false))
        (:then_1
          (CallFunction|SelectAOETiles (Variables|/Game/Actors/Grid/TBS_TileBP.TBS_TileBP_C|GetSouth CurrentTile) (LocalVariables|GetCurrentPath) _returnvalue false false))
        (:then_2
          (CallFunction|SelectAOETiles (Variables|/Game/Actors/Grid/TBS_TileBP.TBS_TileBP_C|GetEast CurrentTile) (LocalVariables|GetCurrentPath) _returnvalue false false))
        (:then_3
          (CallFunction|SelectAOETiles (Variables|/Game/Actors/Grid/TBS_TileBP.TBS_TileBP_C|GetWest CurrentTile) (LocalVariables|GetCurrentPath) _returnvalue false false))))
    (else
      ;[1 1 1] Tile is Valid
      (if (Utilities|IsValid CurrentTile)
        ;[1 1 1] already in list?
        (if (Utilities|Array|ContainsItem Path CurrentTile)
          (return)
          (else
            ;[1 1 1] Check Current Tile Path Length
            (if (and (!= (Utilities|Array|Length (Variables|/Game/Actors/Grid/TBS_TileBP.TBS_TileBP_C|GetTilePath CurrentTile)) 0) (<= (Utilities|Array|Length (Variables|/Game/Actors/Grid/TBS_TileBP.TBS_TileBP_C|GetTilePath CurrentTile)) (Utilities|Array|Length Path)))
              (return)
              (else
                (bind _blocked (CallFunction|SelectTile CurrentTile Occupants%20Block Include%20Occupants))
                (if (not _blocked)
                  (goto _label))))))
        (else
          (return))))))

(fn SelectLineTiles
  (params (StartTile :type TBS%20Tile%20BP%20Object%20Reference) (Direction :type EDirection%20Enum :default "NewEnumerator0") (Amount :type Integer) (SelectSelf :type Boolean) (OccupantsBlock :type Boolean) (IncludeOccupants :type Boolean))
  (LocalVariables|SetCurrentTile StartTile)
  (if SelectSelf
    (CallFunction|SelectTile (LocalVariables|GetCurrentTile) OccupantsBlock IncludeOccupants))
  (for _index (range 1 Amount)
    (switch Utilities|FlowControl|Switch|SwitchonEDirection Direction
      (:NewEnumerator0
        (if (Utilities|IsValid (Variables|/Game/Actors/Grid/TBS_TileBP.TBS_TileBP_C|GetNorth (LocalVariables|GetCurrentTile)))
          (LocalVariables|SetCurrentTile (Variables|/Game/Actors/Grid/TBS_TileBP.TBS_TileBP_C|GetNorth (LocalVariables|GetCurrentTile)))
          (else
            (return))))
      (:NewEnumerator1
        (if (Utilities|IsValid (Variables|/Game/Actors/Grid/TBS_TileBP.TBS_TileBP_C|GetEast (LocalVariables|GetCurrentTile)))
          (LocalVariables|SetCurrentTile (Variables|/Game/Actors/Grid/TBS_TileBP.TBS_TileBP_C|GetEast (LocalVariables|GetCurrentTile)))
          (else
            (return))))
      (:NewEnumerator2
        (if (Utilities|IsValid (Variables|/Game/Actors/Grid/TBS_TileBP.TBS_TileBP_C|GetSouth (LocalVariables|GetCurrentTile)))
          (LocalVariables|SetCurrentTile (Variables|/Game/Actors/Grid/TBS_TileBP.TBS_TileBP_C|GetSouth (LocalVariables|GetCurrentTile)))
          (else
            (return))))
      (:NewEnumerator3
        (if (Utilities|IsValid (Variables|/Game/Actors/Grid/TBS_TileBP.TBS_TileBP_C|GetWest (LocalVariables|GetCurrentTile)))
          (LocalVariables|SetCurrentTile (Variables|/Game/Actors/Grid/TBS_TileBP.TBS_TileBP_C|GetWest (LocalVariables|GetCurrentTile)))
          (else
            (return)))))
    (bind _blocked (CallFunction|SelectTile (LocalVariables|GetCurrentTile) OccupantsBlock IncludeOccupants))
    (if _blocked
      (return)))
  (return))

(fn SelectTilefromTile
  (params (StartTile :type TBS%20Tile%20BP%20Object%20Reference) (XDir :type Integer) (YDir :type Integer) (FacingDir :type EDirection%20Enum :default "NewEnumerator0") (IncludeOccupants :type Boolean%20%28by%20ref%29))
  (LocalVariables|SetCurrentTile StartTile)
  (switch Utilities|FlowControl|Switch|SwitchonEDirection FacingDir
    (:NewEnumerator0
      (LocalVariables|SetXMoveLeft XDir)
      (LocalVariables|SetYMoveLeft YDir))
    (:NewEnumerator1
      (LocalVariables|SetXMoveLeft YDir)
      (bind _result (Utilities|NegateInt XDir)
        (:%20%20
          (LocalVariables|SetYMoveLeft _result))))
    (:NewEnumerator2
      (bind _result_2 (Utilities|NegateInt XDir)
        (:%20%20
          (LocalVariables|SetXMoveLeft _result_2)
          (bind _result_3 (Utilities|NegateInt YDir)
            (:%20%20
              (LocalVariables|SetYMoveLeft _result_3))))))
    (:NewEnumerator3
      (bind _result_4 (Utilities|NegateInt YDir)
        (:%20%20
          (LocalVariables|SetXMoveLeft _result_4)
          (LocalVariables|SetYMoveLeft XDir)))))
  (for _index (range 1 (Math|Integer|Absolute(Integer) (LocalVariables|GetXMoveLeft)))
    (if (> (LocalVariables|GetXMoveLeft) 0)
      (if (Utilities|IsValid (Variables|/Game/Actors/Grid/TBS_TileBP.TBS_TileBP_C|GetEast (LocalVariables|GetCurrentTile)))
        (LocalVariables|SetCurrentTile (Variables|/Game/Actors/Grid/TBS_TileBP.TBS_TileBP_C|GetEast (LocalVariables|GetCurrentTile)))
        (else
          (return)))
      (elif (Utilities|IsValid (Variables|/Game/Actors/Grid/TBS_TileBP.TBS_TileBP_C|GetWest (LocalVariables|GetCurrentTile)))
        (LocalVariables|SetCurrentTile (Variables|/Game/Actors/Grid/TBS_TileBP.TBS_TileBP_C|GetWest (LocalVariables|GetCurrentTile)))
        (else
          (return)))))
  (for _index_2 (range 1 (Math|Integer|Absolute(Integer) (LocalVariables|GetYMoveLeft)))
    (if (> (LocalVariables|GetYMoveLeft) 0)
      (if (Utilities|IsValid (Variables|/Game/Actors/Grid/TBS_TileBP.TBS_TileBP_C|GetNorth (LocalVariables|GetCurrentTile)))
        (LocalVariables|SetCurrentTile (Variables|/Game/Actors/Grid/TBS_TileBP.TBS_TileBP_C|GetNorth (LocalVariables|GetCurrentTile)))
        (else
          (return)))
      (elif (Utilities|IsValid (Variables|/Game/Actors/Grid/TBS_TileBP.TBS_TileBP_C|GetSouth (LocalVariables|GetCurrentTile)))
        (LocalVariables|SetCurrentTile (Variables|/Game/Actors/Grid/TBS_TileBP.TBS_TileBP_C|GetSouth (LocalVariables|GetCurrentTile)))
        (else
          (return)))))
  (CallFunction|SelectTile (LocalVariables|GetCurrentTile) (Class|KismetSystemLibrary|MakeLiteralBool false) IncludeOccupants)
  (return))

(fn AddTiles
  (params (NewTIles :type Array%20of%20TBS%20Tile%20BP%20Object%20References))
  (Utilities|Set|AddItems (Variables|Default|GetTiles) NewTIles))

(fn SetTilesSelectable
  (bind _result (Utilities|Set|ToArray (Variables|Default|GetSelectedTiles)))
  (for _array_element _result
    (if (Utilities|IsValid _array_element)
      (Default|SetSelectable _array_element true))))

(fn RemoveTiles
  (params (TilesIn :type Set%20of%20TBS%20Tile%20BP%20Object%20References))
  (bind _result (Utilities|Set|ToArray TilesIn))
  (Utilities|Set|RemoveItems (Variables|Default|GetTiles) _result))

(fn SelectTile
  (params (TIle :type TBS%20Tile%20BP%20Object%20Reference) (OccupantsBlock :type Boolean%20%28by%20ref%29) (IncludeOccupants :type Boolean%20%28by%20ref%29))
  ;[1 1 1] Check if Valid Tile
  (if (Variables|/Game/Actors/Grid/TBS_TileBP.TBS_TileBP_C|GetisFalling TIle)
    (return false false)
    (else
      ;[1 1 1] Check if Occupied
      (if (Utilities|IsValid (Variables|/Game/Actors/Grid/TBS_TileBP.TBS_TileBP_C|GetOccupant TIle))
        ;[1 1 1] Check if actor can be damaged- if not its not selectable
        (if (Variables|/Game/Actors/TBS_ActorBP.TBS_ActorBP_C|GetisDamageable (Variables|/Game/Actors/Grid/TBS_TileBP.TBS_TileBP_C|GetOccupant TIle))
          ;[1 1 1] Check if we add tiles with occupants
          (if IncludeOccupants
            (Utilities|Set|Add (Variables|Default|GetSelectedTiles) TIle)
            (return OccupantsBlock true)
            (else
              (return OccupantsBlock false)))
          (else
            ;[1 1 1] Always Block - Never Add
            (return true false)))
        (else
          ;[1 1 1] Not Occupied - Add Tile
          (Utilities|Set|Add (Variables|Default|GetSelectedTiles) TIle)
          (return false true))))))